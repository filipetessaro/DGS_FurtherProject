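; Destructible double sliding door in the BallisticsVFX demo map that opens on trigger overlap and closes when the overlap ends.
; Each leaf slides sideways with an eased MoveComponentTo, using an in-motion flag and a short Delay retry loop to avoid overlapping moves.
; A fractured leaf stops accepting new moves and increments the player character's AssholeRating and DoorsDestroyed counters.
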(event `self.Trigger_1.OnComponentBeginOverlap`
  (params (OverlappedComponent :type "PrimitiveComponent Object Reference") (OtherActor :type "Actor Object Reference") (OtherComp :type "PrimitiveComponent Object Reference") (OtherBodyIndex :type Integer) (bFromSweep :type Boolean) (SweepResult :type "HitResult Structure (by ref)"))
  (`|ExecutionSequence`
    (:`then_0`
      (if (not (`self.Left Door Is broken!`))
        (if (`self.InMotionLeft`) :!label _label
          (`KismetSystemLibrary.Delay` 0.25)
          (goto _label)
          (else
            (set `self.InMotionLeft` true)
            (`KismetSystemLibrary.MoveComponentTo` (`self.SM_Door_DM_left`) (0.0 180.0 0.0) (struct) true true 1.0)
            (set `self.InMotionLeft` false)))))
    (:`then_1`
      (if (not (`self.Right Door Is broken!`))
        (if (`self.InMotionRight`) :!label _label_2
          (`KismetSystemLibrary.Delay` 0.25)
          (goto _label_2)
          (else
            (set `self.InMotionRight` true)
            (`KismetSystemLibrary.MoveComponentTo` (`self.SM_Door_DM_right`) (0.0 -180.0 0.0) (struct :`Yaw` -180.0) true true 1.0)
            (set `self.InMotionRight` false)))))))

(event `self.SM_Door_DM_left.OnComponentFracture`
  (params (HitPoint :type "Vector Structure (by ref)") (HitDirection :type "Vector Structure (by ref)"))
  (bind _output_get (set `self.Left Door Is broken!` true))
  (if _output_get
    (bind _asfirst_person_character_rifle_2 (cast `/Game/Packs/BallisticsVFX/FirstPersonBPExamples/FirstPersonCharacter_rifle_2` (`GameplayStatics.GetPlayerCharacter` 0) :!label _label_3))
    (set `/Game/Packs/BallisticsVFX/FirstPersonBPExamples/FirstPersonCharacter_rifle_2.AssholeRating` (+ (`/Game/Packs/BallisticsVFX/FirstPersonBPExamples/FirstPersonCharacter_rifle_2.AssholeRating` _asfirst_person_character_rifle_2) 1.0) _asfirst_person_character_rifle_2)
    (set `/Game/Packs/BallisticsVFX/FirstPersonBPExamples/FirstPersonCharacter_rifle_2.Doors Destroyed?` (+ (`/Game/Packs/BallisticsVFX/FirstPersonBPExamples/FirstPersonCharacter_rifle_2.Doors Destroyed?` _asfirst_person_character_rifle_2) 1.0) _asfirst_person_character_rifle_2)))

(event `self.SM_Door_DM_right.OnComponentFracture`
  (params (HitPoint :type "Vector Structure (by ref)") (HitDirection :type "Vector Structure (by ref)"))
  (bind _output_get (set `self.Right Door Is broken!` true))
  (if _output_get
    (goto _label_3)))

(event `self.Trigger_1.OnComponentEndOverlap`
  (params (OverlappedComponent :type "PrimitiveComponent Object Reference") (OtherActor :type "Actor Object Reference") (OtherComp :type "PrimitiveComponent Object Reference") (OtherBodyIndex :type Integer))
  (`|ExecutionSequence`
    (:`then_0`
      (if (not (`self.Left Door Is broken!`))
        (if (`self.InMotionLeft`) :!label _label_4
          (`KismetSystemLibrary.Delay` 0.25)
          (goto _label_4)
          (else
            (set `self.InMotionLeft` true)
            (`KismetSystemLibrary.MoveComponentTo` (`self.SM_Door_DM_left`) (0.0 0.0 0.0) (struct) true true 1.0)
            (set `self.InMotionLeft` false)))))
    (:`then_1`
      (if (not (`self.Right Door Is broken!`))
        (if (`self.InMotionRight`) :!label _label_5
          (`KismetSystemLibrary.Delay` 0.25)
          (goto _label_5)
          (else
            (set `self.InMotionRight` true)
            (`KismetSystemLibrary.MoveComponentTo` (`self.SM_Door_DM_right`) (0.0 0.0 0.0) (struct :`Yaw` -180.0) true true 1.0)
            (set `self.InMotionRight` false)))))))

(fn `UserConstructionScript`
  (set `self.Left Door Is broken!` false)
  (set `self.Right Door Is broken!` false))