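; BP_DoorRoomsEntry is an interactive door that the player opens and closes with the E key.
; Overlapping the Collision component enables the player's input on the actor, and leaving it disables that input.
; E plays or reverses a timeline depending on whether its current DoorRoot value is above -1.
; The timeline update applies DoorRoot as the relative yaw of the DoorMetal component.
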(event `self.Collision.OnComponentBeginOverlap`
  (params (OverlappedComponent :type "PrimitiveComponent Object Reference") (OtherActor :type "Actor Object Reference") (OtherComp :type "PrimitiveComponent Object Reference") (OtherBodyIndex :type Integer) (bFromSweep :type Boolean) (SweepResult :type "HitResult Structure (by ref)"))
  (`self.EnableInput` (`GameplayStatics.GetPlayerController` 0)))

(event `Key|E`
  (params (Key :type "Key Structure"))
  (:`Pressed`
    (if (> (stale _door_root) -1.0)
      (bind (_direction _door_root) (`Timeline|Línea de tiempo_1` :!label _label)
        (:`Update`
          (`SceneComponent.K2_SetRelativeRotation` (`self.DoorMetal`) (`KismetMathLibrary.MakeRotator` 0.0 0.0 _door_root) false false)))
      (else
        (goto _label :!via `Reverse`)))))

(event `self.Collision.OnComponentEndOverlap`
  (params (OverlappedComponent :type "PrimitiveComponent Object Reference") (OtherActor :type "Actor Object Reference") (OtherComp :type "PrimitiveComponent Object Reference") (OtherBodyIndex :type Integer))
  (`self.DisableInput` (`GameplayStatics.GetPlayerController` 0)))

(fn `UserConstructionScript`)