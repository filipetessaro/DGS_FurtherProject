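; Base player character that handles movement, jumping, first/third-person camera switching and inventory-based merchant trading.
; Movement and look input are gated by UI states, with rotation mode following camera and equipped weapon, and zoom driving the spring arm or book reader.
; Authority starts health and stamina regen and computes aim pitch, which clients request through ServerSetPitch.
; Purchases check money and encumbrance, while sales pay half price.
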(event `self.ReceiveBeginPlay`
  (bind _returnvalue (`GameplayStatics.GetPlayerController` 0))
  (bind _healthstaminacomponent (`self.HealthStaminaComponent`))
  ;[1 1 1] Begin play to initiate Regen functions and add HUD
  (`parent.ReceiveBeginPlay`)
  (`/Engine/EditorBlueprintResources/ActorMacros.Switch Has Authority`
    (:`Authority`
      (`/Game/Blueprints/BPC_RegenComponent.StartHealthRegen` _healthstaminacomponent false 5.0)
      (`/Game/Blueprints/BPC_RegenComponent.StartStaminaRegen` _healthstaminacomponent false 5.0))
    (:`Remote`
      _))
  (`KismetArrayLibrary.Array_Add` (`SceneCaptureComponent.ShowOnlyActors` (`self.SceneCaptureComponent2D`)) self)
  (`KismetSystemLibrary.Delay` 0.2)
  (set `PlayerController.bShowMouseCursor` false _returnvalue)
  (`WidgetBlueprintLibrary.SetInputMode_GameOnly` _returnvalue))

(event `InputAxis|MoveForward`
  (params (AxisValue :type "Float (single-precision)"))
  (bind _returnvalue (> 0.0 0.5))
  ;[1 1 1] Player movement
  (if (not (or (`self.InventoryOpened?`) (`self.MerchantOpened?`)))
    (`self.AddMovementInput` (`KismetMathLibrary.GetForwardVector` (`KismetMathLibrary.MakeRotator` 0.0 0.0 (.yaw (`self.GetControlRotation`)))) AxisValue)
    (if (`self.IsFirstPerson`)
      ;[1 1 1] Headbob
      (if (`self.Aiming`)
        (set `self.HeadBobScale` 0.0)
        (else
          (set `self.HeadBobScale` 1.0)))
      (if _returnvalue
        (`PlayerController.ClientStartCameraShake` :`self` (`GameplayStatics.GetPlayerController` 0) :`Shake` "/Game/Packs/BallisticsVFX/FirstPersonBPExamples/HeadBobShake.HeadBobShake_C" :`Scale` (* (`self.HeadBobScale`) (`KismetMathLibrary.Lerp` 1.0 0.0 (stale _0_1_in_a_second))))
        (if (not _returnvalue)
          (bind (_direction _0_1_in_a_second) (`Timeline|Timeline_0_0`)))))))

(event `InputAxis|MoveRight`
  (params (AxisValue :type "Float (single-precision)"))
  ;[1 1 1] Player movement
  (if (not (or (`self.InventoryOpened?`) (`self.MerchantOpened?`)))
    (`self.AddMovementInput` (`KismetMathLibrary.GetRightVector` (`KismetMathLibrary.MakeRotator` 0.0 0.0 (.yaw (`self.GetControlRotation`)))) AxisValue)))

(event `InputAxis|Turn`
  (params (AxisValue :type "Float (single-precision)"))
  ;[1 1 1] Player movement
  (bind _output_get (set `self.TurnScale` AxisValue))
  (if (`self.Inspecting/ReadingItem?`)
    _
    (elif (`self.IsFirstPerson`)
      (`self.AddControllerYawInput` (* AxisValue (* (`self.BaseTurnRate`) (`GameplayStatics.GetGlobalTimeDilation`)) (`GameplayStatics.GetWorldDeltaSeconds`)))
      (else
        (`self.AddControllerYawInput` _output_get)))))

(event `ServerSetPitch`
  ;[1 1 1] Player movement
  (`/Engine/EditorBlueprintResources/ActorMacros.Switch Has Authority`
    (:`Authority`
      (`self.SetPitchAxis`))))

(event `InputAction|ToggleCamera`
  (params (Key :type "Key Structure"))
  (bind _charactermovement (`self.CharacterMovement`))
  ;[1 1 1] Camera toggle
  (:`Pressed`
    (if (`self.IsFirstPerson`)
      (set `self.IsFirstPerson` false)
      (`ActorComponent.Deactivate` (`self.FirstPersonCamera`))
      (`ActorComponent.Activate` (`self.Camera`) true)
      (`/Engine/EditorBlueprintResources/StandardMacros.IsValid` (`self.WeaponSlot`) :!label _label
        (:`Is Valid`
          (set `self.bUseControllerRotationYaw` true)
          (set `CharacterMovementComponent.bOrientRotationToMovement` false (`self.CharacterMovement`)))
        (:`Is Not Valid`
          (set `self.bUseControllerRotationYaw` false)
          (set `CharacterMovementComponent.bOrientRotationToMovement` true _charactermovement)))
      (else
        (set `self.IsFirstPerson` true)
        (`ActorComponent.Deactivate` (`self.Camera`))
        (`ActorComponent.Activate` (`self.FirstPersonCamera`) true)
        (set `self.bUseControllerRotationYaw` true)
        (set `CharacterMovementComponent.bOrientRotationToMovement` false _charactermovement)))))

(event `InputAxis|LookUp`
  (params (AxisValue :type "Float (single-precision)"))
  ;[1 1 1] Player movement
  (bind _output_get (set `self.LookUpScale` AxisValue))
  (if (not (`self.Inspecting/ReadingItem?`))
    (`/Engine/EditorBlueprintResources/ActorMacros.Switch Has Authority`
      (:`Authority`
        (`self.SetPitchAxis`))
      (:`Remote`
        (`self.ServerSetPitch`)))
    (if (`self.IsFirstPerson`)
      (`self.AddControllerPitchInput` (* AxisValue (* (`self.BaseLookUpRate`) (`GameplayStatics.GetGlobalTimeDilation`)) (`GameplayStatics.GetWorldDeltaSeconds`)))
      (else
        (`self.AddControllerPitchInput` _output_get)))))

(event `ExternalVeiifyCamera`
  ;[1 1 1] Camera toggle
  (goto _label))

(event `InputAction|Jump`
  (params (Key :type "Key Structure"))
  ;[1 1 1] Player movement
  (:`Pressed`
    (`self.Jump`)))

(event `self.ReceiveTick`
  (params (DeltaSeconds :type "Float (single-precision)"))
  (`parent.ReceiveTick` DeltaSeconds))

(event `InputAction|ZoomIn`
  (params (Key :type "Key Structure"))
  (bind _w_bookreadwidget (`/Game/Blueprints/Core/F_GameInstance.W_BookReadWidget` (`self.GameInstanceRef`)))
  ;[1 1 1] TP Zoom / Book zoom
  (:`Pressed`
    (if (`self.IsFirstPerson`)
      _
      (elif (not (`self.MerchantOpened?`))
        (set `self.Zoom` (`KismetMathLibrary.FClamp` (- (`self.Zoom`) 10.0) 120.0 300.0))
        (if (`self.InventoryOpened?`)
          (`/Engine/EditorBlueprintResources/StandardMacros.IsValid` _w_bookreadwidget :!label _label_2
            (:`Is Valid`
              (`/Game/Blueprints/Inventory/W_BookReadInspectView.ZoomIn/Out` _w_bookreadwidget (`self.Zoom`))))
          (else
            (set `SpringArmComponent.TargetArmLength` (`KismetMathLibrary.FClamp` (- (`SpringArmComponent.TargetArmLength` (`self.ThirdPersonArm`)) 10.0) 50.0 600.0) (`self.ThirdPersonArm`))))))))

(event `InputAction|ZoomOut`
  (params (Key :type "Key Structure"))
  ;[1 1 1] TP Zoom / Book zoom
  (:`Pressed`
    (if (`self.IsFirstPerson`)
      _
      (elif (not (`self.MerchantOpened?`))
        ;;[1 1 1] for the read book
        (set `self.Zoom` (`KismetMathLibrary.FClamp` (+ (`self.Zoom`) 10.0) 120.0 300.0))
        (if (`self.InventoryOpened?`)
          (goto _label_2)
          (else
            (set `SpringArmComponent.TargetArmLength` (`KismetMathLibrary.FClamp` (+ (`SpringArmComponent.TargetArmLength` (`self.ThirdPersonArm`)) 10.0) 50.0 600.0) (`self.ThirdPersonArm`))))))))

(event `Key|NumPadTwo`
  (params (Key :type "Key Structure"))
  (:`Pressed`
    (`self.LaunchCharacter` (0.0 0.0 2000.0) false true)))

(fn `PlayerBuyItem`
  (params (Item :type "/Game/Blueprints/items/S_ItemData Structure"))
  (bind (_itemname _itemdescription _icon _questitem_ _itemtype _isstackable_ _weight _pricevalue) (break `/Game/Blueprints/items/S_ItemData` Item))
  (bind _s_characterdata (`self.S_CharacterData`))
  (bind (_charname _charicon _encumbance _totalweight _level _experience _money) (break `/Game/Blueprints/Datas/S_CharacterData` _s_characterdata))
  (if (>= _money _pricevalue)
    (if (>= _totalweight _encumbance)
      (`KismetSystemLibrary.PrintString` "YOU ARE TOO HEAVY")
      (else
        (setmembers `/Game/Blueprints/Datas/S_CharacterData` :`StructRef` _s_characterdata :`Money` (`KismetMathLibrary.FClamp` (- _money _pricevalue) 0.0 1000000000.0))
        (`self.AddSpecificItemToInventory` Item)
        (`self.ExternalUpdateInventory/Merchant`)))
    (else
      (`KismetSystemLibrary.PrintString` "YOU DON´T HAVE ENOUGHT MONEY")))
  (return))

(fn `PlayerSellItem`
  (params (Item :type "Array of /Game/Blueprints/items/S_ItemData Structure") (Index :type Integer) (ItemWeight :type "Float (double-precision)") (PriceValue :type "Float (double-precision)"))
  (bind _s_characterdata (`self.S_CharacterData`))
  (setmembers `/Game/Blueprints/Datas/S_CharacterData` :`StructRef` _s_characterdata :`Money` (+ (`.Money_22_20A961FB4A1B2AF9B1C6E28385C73C60` (break `/Game/Blueprints/Datas/S_CharacterData` _s_characterdata)) (/ PriceValue 2.0)))
  (`self.RemoveItemFromInventory` Item Index ItemWeight)
  (`self.ExternalUpdateInventory/Merchant`)
  (return))

(fn `SetPitchAxis`
  (bind (_returnvalue_roll _returnvalue_pitch) (`KismetMathLibrary.BreakRotator` (`KismetMathLibrary.NormalizedDeltaRotator` (`self.GetControlRotation`) (`self.K2_GetActorRotation`))))
  (set `self.PitchAxis` _returnvalue_pitch))

(fn `UserConstructionScript`)