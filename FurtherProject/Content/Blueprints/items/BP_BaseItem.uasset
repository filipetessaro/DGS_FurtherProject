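; Base actor for inventory items, with a pickup prompt, custom-depth highlight and an inspect view.
; Inspection swaps the item mesh for a rotatable copy, filmed by a SceneCapture2D that shows only this actor, with orthographic zoom.
; UseItem branches on item type to equip weapons, armor or shields, open the read/inspect screen through the game instance, or consume.
; Consumables and food apply data-table health, stamina or stat effects, then leave the inventory and destroy themselves.
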(event `self.ReceiveBeginPlay`
  ;[0.06646 1 0] BeginPlay to setup 2d camera actor to see
  ; and setup widget info
  (setmembers `/Game/Blueprints/items/S_ItemData` :`StructRef` (`self.S_ItemData`) :`SelfRef` self)
  (`KismetArrayLibrary.Array_Add` (`SceneCaptureComponent.ShowOnlyActors` (`self.SceneCaptureComponent2D`)) self)
  (`StaticMeshComponent.SetStaticMesh` (`self.InspectMesh`) (`StaticMeshComponent.StaticMesh` (`self.ItemMesh`)))
  (bind _asw_item_message (cast `/Game/Blueprints/Inventory/W_ItemMessage` (`WidgetComponent.GetUserWidgetObject` (`self.Widget`))))
  (set `/Game/Blueprints/Inventory/W_ItemMessage.TextToShow` "Press \"E\" To Pick Up" _asw_item_message))

(event `OnItemPìckedUp`
  ;[1 1 1] Use / Interact system
)

(event `AddRotation`
  (params (`Delta Rotation Y (Pitch)` :type "Float (double-precision)") (`Delta Rotation Z (Yaw)` :type "Float (double-precision)"))
  ;[1 1 1] Inspect system
  (`SceneComponent.K2_AddRelativeRotation` (`self.InspectMesh`) (`KismetMathLibrary.MakeRotator` (`KismetMathLibrary.FClamp` (* `Delta Rotation Y (Pitch)` 3.0) -15.0 150.0) (`KismetMathLibrary.FClamp` (* `Delta Rotation Z (Yaw)` -3.0) -15.0 15.0)) false false))

(event `StartInspectSystem`
  (bind _scenecapturecomponent2d (`self.SceneCaptureComponent2D`))
  ;[1 1 1] Inspect system
  (`SceneComponent.SetVisibility` (`self.ItemMesh`) false false)
  (`SceneComponent.SetVisibility` (`self.InspectMesh`) true false)
  (`ActorComponent.Activate` _scenecapturecomponent2d true)
  (set `SceneCaptureComponent.bCaptureEveryFrame` true _scenecapturecomponent2d))

(event `UseItem`
  (params (UserActor :type "/Game/Blueprints/BP_BaseCharacter Object Reference") (`Inspect?` :type Boolean))
  (bind (_itemname _itemdescription _icon _questitem_ _itemtype) (break `/Game/Blueprints/items/S_ItemData` (`self.S_ItemData`)))
  ;[1 1 1] Use / Interact system
  (`GameplayStatics.PlaySound2D` (select `/Game/Blueprints/items/E_ItemType` _itemtype :!type "SoundBase Object Reference") 1.0 1.0 0.0 null null)
  (if `Inspect?`
    (`self.ReadBook/InspectItem` self)
    (else
      (switch `/Game/Blueprints/items/E_ItemType` _itemtype
        (:`NewEnumerator3`
          (`self.ConsumeItem` UserActor :!label _label))
        (:`NewEnumerator0`
          (`/Game/Blueprints/BP_BaseCharacter.UpdateWeapon` UserActor (cast `/Game/Blueprints/items/Weapons/BP_WeaponBase` self :!pure true)))
        (:`NewEnumerator1`
          (`/Game/Blueprints/BP_BaseCharacter.UpdateArmor` UserActor (cast `/Game/Blueprints/items/Armors/BP_ArmorBase` self :!pure true)))
        (:`NewEnumerator2`
          (`/Game/Blueprints/BP_BaseCharacter.UpdateShield` UserActor (cast `/Game/Blueprints/items/Shields/BP_ShieldBase` self :!pure true)))
        (:`NewEnumerator5`
          (goto _label))
        (:`NewEnumerator6`
          (`self.ReadBook/InspectItem` (cast `/Game/Blueprints/items/Books/BP_BookBase` self :!pure true)))))))

(event `BookZoom`
  (params (Zoom :type "Float (double-precision)"))
  ;[1 1 1] Inspect system
  (set `SceneCaptureComponent2D.OrthoWidth` (`KismetMathLibrary.FClamp` Zoom 120.0 300.0) (`self.SceneCaptureComponent2D`)))

(event `SetMessageVisible`
  (`SceneComponent.SetVisibility` (`self.Widget`) true false)
  (`PrimitiveComponent.SetRenderCustomDepth` (`self.ItemMesh`) true))

(event `SetMessageInvisible`
  (`SceneComponent.SetVisibility` (`self.Widget`) false false)
  (`PrimitiveComponent.SetRenderCustomDepth` (`self.ItemMesh`) false))

(fn `ConsumeItem`
  (params (User :type "/Game/Blueprints/BP_BaseCharacter Object Reference"))
  (bind _healthstaminacomponent (`/Game/Blueprints/BP_BaseCharacter.HealthStaminaComponent` User))
  (bind _returnvalue (`|GetDataTableRow` "/Game/Blueprints/items/DT_ItemsEffects.DT_ItemsEffects" (`KismetStringLibrary.Conv_StringToName` (`|GetEnumeratorNameAsString` (`self.S_ConsumableEffect`))))
    (:`then`
      (bind (_itemname _selecteffect _value) (break `/Game/Blueprints/items/S_ItemEffectsList` _returnvalue))
      (switch `/Game/Blueprints/items/E_EffectsList` _selecteffect
        (:`NewEnumerator0`
          (`/Game/Blueprints/BPC_RegenComponent.RestoreHealth` _healthstaminacomponent _value))
        (:`NewEnumerator1`
          (`/Game/Blueprints/BPC_RegenComponent.RestoreStamina` _healthstaminacomponent _value))
        (:`NewEnumerator2`
          (`/Game/Blueprints/BP_BaseCharacter.UpdateStatus` User "NewEnumerator1" _value))
        (:`NewEnumerator3`
          (`/Game/Blueprints/BP_BaseCharacter.UpdateStatus` User "NewEnumerator0" _value)))
      (`/Game/Blueprints/BP_BaseCharacter.RemoveItemFromInventory` User (`/Game/Blueprints/BP_BaseCharacter.S_InventoryData` User) (`/Game/Blueprints/BP_BaseCharacter.InventoryButtonClicked` User) 0.0)
      (`self.K2_DestroyActor`))))

(fn `HideItem`
  (bind _itemmesh (`self.ItemMesh`))
  (`self.SetActorEnableCollision` false)
  (`self.SetActorHiddenInGame` true)
  (`PrimitiveComponent.SetSimulatePhysics` _itemmesh false)
  (`PrimitiveComponent.SetCollisionEnabled` _itemmesh "NoCollision"))

(fn `ReadBook/InspectItem`
  (params (ItemRef :type "/Game/Blueprints/items/BP_BaseItem Object Reference"))
  (bind _itemmesh (`/Game/Blueprints/items/BP_BaseItem.ItemMesh` ItemRef))
  (`PrimitiveComponent.SetSimulatePhysics` _itemmesh false)
  (`PrimitiveComponent.SetCollisionEnabled` _itemmesh "NoCollision")
  (bind _asf_game_instance (cast `/Game/Blueprints/Core/F_GameInstance` (`GameplayStatics.GetGameInstance`)))
  (`/Game/Blueprints/Core/F_GameInstance.AddBookRead/InspectScreen` _asf_game_instance ItemRef)
  (return))

(fn `UserConstructionScript`)