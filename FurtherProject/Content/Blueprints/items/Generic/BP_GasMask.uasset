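; BP_GasMask is a gas mask item actor whose look is configured per instance in the Construction Script.
; The Flat option swaps the static mesh to a flat variant.
; A dynamic instance of M_GasMask receives the light color and intensity, with LightEnabled converted to a float multiplier that zeroes intensity when off.
; The event graph has no active logic.
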(fn `UserConstructionScript`
  ;[0.05967 0.3863 1] Set Mesh (Flat/Normal) and audjust material parameters
  (`|ExecutionSequence`
    (:`then_0`
      (if (`self.Flat`)
        (`StaticMeshComponent.SetStaticMesh` (`self.SM_GasMask`) "/Game/Assets/3D_Assets/SurvivalAssetPack/Meshes/SM_GasMask-Flat.SM_GasMask-Flat")))
    (:`then_1`
      (bind _returnvalue (`PrimitiveComponent.CreateDynamicMaterialInstance` (`self.SM_GasMask`) 0 "/Game/Assets/3D_Assets/SurvivalAssetPack/Materials/M_GasMask.M_GasMask" "None"))
      (`MaterialInstanceDynamic.SetVectorParameterValue` _returnvalue "LightColor" (`self.Light Color`))
      (`MaterialInstanceDynamic.SetScalarParameterValue` _returnvalue "LightIntensity" (* (`self.Light Intensity`) (`KismetMathLibrary.Conv_BoolToDouble` (`self.Light Enabled`))))
      (`PrimitiveComponent.SetMaterial` (`self.SM_GasMask`) 0 _returnvalue))))