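; BP_GasStove is a gas stove prop whose flames and gas sound follow its Enabled setting.
; The construction script shows or hides every particle system component according to Enabled.
; It plays the gas sound only when both Enabled and HasSound are true, otherwise stopping it and zeroing its volume multiplier.
; The event graph holds only disabled placeholder events, so it has no runtime toggle logic.
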(fn `UserConstructionScript`
  (bind _s_gassound (`self.S_GasSound`))
  (bind _enabled (`self.Enabled`))
  (`|ExecutionSequence`
    (:`then_0`
      ;[0.2621 0.4044 1] Show/Hide Flames
      (for _array_element (`self.K2_GetComponentsByClass` "/Script/Engine.ParticleSystemComponent")
        (`SceneComponent.SetHiddenInGame` _array_element (not _enabled) false)
        (`SceneComponent.SetVisibility` _array_element _enabled false)))
    (:`then_1`
      ;[0.1669 0.4103 1] Play the needed Sound file
      (if (and (`self.HasSound`) (`self.Enabled`))
        (`AudioComponent.Play` (`self.S_GasSound`) 0.0)
        (else
          (`AudioComponent.Stop` _s_gassound)
          (`AudioComponent.SetVolumeMultiplier` _s_gassound 0.0))))))