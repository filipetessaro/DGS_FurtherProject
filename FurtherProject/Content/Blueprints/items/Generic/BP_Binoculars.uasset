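; BP_Binoculars is a binoculars item actor whose lens or indicator light color and brightness are configurable per instance.
; Its Construction Script creates a dynamic instance of M_Binoculars for the SMBinocular mesh, feeding in LightColor and LightIntensity, with LightEnabled multiplied in as a zero-or-one switch.
; The event graph is empty, so it has no runtime logic.
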(fn `UserConstructionScript`
  (bind _returnvalue (`PrimitiveComponent.CreateDynamicMaterialInstance` (`self.SM_Binocular`) 0 "/Game/Assets/3D_Assets/SurvivalAssetPack/Materials/M_Binoculars.M_Binoculars" "None"))
  (`MaterialInstanceDynamic.SetVectorParameterValue` _returnvalue "LightColor" (`self.Light Color`))
  (`MaterialInstanceDynamic.SetScalarParameterValue` _returnvalue "LightIntensity" (* (`self.Light Intensity`) (`KismetMathLibrary.Conv_BoolToDouble` (`self.Light Enabled`))))
  (`PrimitiveComponent.SetMaterial` (`self.SM_Binocular`) 0 _returnvalue))