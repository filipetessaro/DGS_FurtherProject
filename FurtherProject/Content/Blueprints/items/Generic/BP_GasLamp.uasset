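; BP_GasLamp is a configurable gas lamp prop with an enable toggle, color, intensity and optional gas sound.
; The construction script does all the work, driving the glow through a dynamic material instance on the mesh's second material slot.
; Intensity is split between shadowed and unshadowed point lights by SelfShadowDensity to tune self-shadow strength.
; The sound plays only when enabled and wanted, otherwise it is stopped and muted.
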(fn `UserConstructionScript`
  (bind _sm_gaslamp (`self.SM_GasLamp`))
  (bind _s_gassound (`self.S_GasSound`))
  (bind _returnvalue (* (`KismetMathLibrary.Conv_BoolToDouble` (`self.Enabled`)) (`self.Intensity`)))
  ;[0.1073 0.4932 1] Set Material and Spotlight Parameters
  (bind _returnvalue_2 (`PrimitiveComponent.CreateDynamicMaterialInstance` _sm_gaslamp 1 (`PrimitiveComponent.GetMaterial` _sm_gaslamp 1) "None"))
  (`MaterialInstanceDynamic.SetVectorParameterValue` _returnvalue_2 "LightColor" (`self.Color`))
  (`MaterialInstanceDynamic.SetScalarParameterValue` _returnvalue_2 "LightIntensity" (/ _returnvalue 100.0))
  (`PrimitiveComponent.SetMaterial` (`self.SM_GasLamp`) 1 _returnvalue_2)
  (`LightComponent.SetIntensity` (`self.PointLight`) (* (- 1.0 (`self.SelfShadowDensity`)) _returnvalue))
  (`LightComponent.SetIntensity` (`self.PointLight_WithShadow`) (* (`self.SelfShadowDensity`) _returnvalue))
  (`LightComponent.SetLightColor` (`self.PointLight`) (`self.Color`) true)
  (`LightComponent.SetLightColor` (`self.PointLight_WithShadow`) (`self.Color`) true)
  (if (`self.HasSound`)
    (if (`self.Enabled`)
      (`AudioComponent.Play` _s_gassound 0.0)
      (else
        (`AudioComponent.Stop` _s_gassound :!label _label)
        (`AudioComponent.SetVolumeMultiplier` _s_gassound 0.0) ; kill existing sound instances
      ))
    (else
      (goto _label))))