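; Base candle actor with a flame particle effect and lights that show at nightfall and hide at sunrise.
; It binds to day/night dispatchers on F_GameInstance to toggle the particle system, point light and shadow light.
; After a random startup delay, a timeline drives the point light's intensity to create flicker, staggering candles from one another.
; The construction script stores a dynamic instance of the particle material.
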(event `self.ReceiveBeginPlay`
  (bind _asf_game_instance (cast `/Game/Blueprints/Core/F_GameInstance` (`GameplayStatics.GetGameInstance`)))
  (add `/Game/Blueprints/Core/F_GameInstance.CallSunRise` _asf_game_instance (delegate `CallSunRise_Event_0`))
  (add `/Game/Blueprints/Core/F_GameInstance.CallNightFall` _asf_game_instance (delegate `CallNightFall_Event_0`))
  (`KismetSystemLibrary.Delay` (`KismetMathLibrary.RandomFloatInRange` 1.5 5.0))
  ;[1 1 1] Creates the flickering effect
  (bind (_direction _intensitymultiplier) (`Timeline|Flickering` :!via `PlayFromStart`)
    (:`Update`
      (`LightComponent.SetIntensity` (`self.PointLight`) (* 3000.0 _intensitymultiplier)))))

(event `CallSunRise_Event_0`
  ;[1 1 1] turn on / off based on
  ; time of day/night
  (`SceneComponent.SetVisibility` (`self.ParticleSystem`) false false)
  (`SceneComponent.SetVisibility` (`self.PointLight`) false false)
  (`SceneComponent.SetVisibility` (`self.ShadowLight`) false false))

(event `CallNightFall_Event_0`
  ;[1 1 1] turn on / off based on
  ; time of day/night
  (`SceneComponent.SetVisibility` (`self.ShadowLight`) true false)
  (`SceneComponent.SetVisibility` (`self.PointLight`) true false)
  (`SceneComponent.SetVisibility` (`self.ParticleSystem`) true false))

(fn `UserConstructionScript`
  (bind _particlesystem (`self.ParticleSystem`))
  (bind _returnvalue (`PrimitiveComponent.CreateDynamicMaterialInstance` _particlesystem 0 (`PrimitiveComponent.GetMaterial` _particlesystem 0) "None"))
  (set `self.CandleMaterialInst` _returnvalue))