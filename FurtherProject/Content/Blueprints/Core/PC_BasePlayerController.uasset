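; Base player controller that sets game-only input and sets up each player's pawn and HUD on BeginPlay.
; With authority, a local controller creates the HUD widget for its existing character.
; The remote branch calls SwapCharacterForClient, which replaces the pawn with a BP_PlayerBaseDog at a random PlayerStart and possesses it.
; After a short delay, that branch asks the new pawn, if valid, to create its HUD.
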(event `self.ReceiveBeginPlay`
  (bind _returnvalue (`self.K2_GetPawn`))
  (bind _newpawn (`self.NewPawn`))
  (set `self.bShowMouseCursor` false)
  (`WidgetBlueprintLibrary.SetInputMode_GameOnly` self)
  (bind _outactors (`GameplayStatics.GetAllActorsOfClass` "/Script/Engine.PlayerStart"))
  (set `self.SpawnPoints` _outactors)
  (`/Engine/EditorBlueprintResources/ActorMacros.Switch Has Authority`
    (:`Authority`
      (if (`self.IsLocalController`)
        (`/Engine/EditorBlueprintResources/StandardMacros.IsValid` _returnvalue
          (:`Is Valid`
            (bind _returnvalue_2 (`|CreateWidget` "/Game/Menus/W_HUD_Widget.W_HUD_Widget_C" self (cast `/Game/Blueprints/BP_BaseCharacter` _returnvalue :!pure true)))
            (`UserWidget.AddToViewport` _returnvalue_2 0)))))
    (:`Remote`
      (`self.SwapCharacterForClient`)
      (`KismetSystemLibrary.Delay` 0.2)
      (`/Engine/EditorBlueprintResources/StandardMacros.IsValid` _newpawn
        (:`Is Valid`
          (`/Game/Blueprints/BP_PlayerBaseDog.CreateHUD` _newpawn))))))

(event `SwapCharacterForClient`
  (bind _returnvalue (`self.K2_GetPawn`))
  (bind _spawnpoints (`self.SpawnPoints`))
  (`/Engine/EditorBlueprintResources/StandardMacros.IsValid` _returnvalue
    (:`Is Valid`
      (`self.K2_DestroyActor` _returnvalue))
    (:`Is Not Valid`
      _))
  (bind _returnvalue_2 (`|SpawnActorFromClass` "/Game/Blueprints/BP_PlayerBaseDog.BP_PlayerBaseDog_C" (`self.GetTransform` (`|GetArrayItem` _spawnpoints (`KismetMathLibrary.RandomIntegerInRange` 0 (- (`KismetArrayLibrary.Array_Length` _spawnpoints) 1)))) "AdjustIfPossibleButAlwaysSpawn" "OverrideRootScale" null null))
  (set `self.NewPawn` _returnvalue_2)
  (`self.Possess` (`self.NewPawn`)))

(fn `UserConstructionScript`)