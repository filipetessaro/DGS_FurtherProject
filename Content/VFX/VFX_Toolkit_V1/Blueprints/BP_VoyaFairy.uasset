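; BP_VoyaFairy is an animated fairy effect actor from the VFX Toolkit that also drives a material time parameter.
; On BeginPlay, the Faketicker timeline adds local yaw to two arm components on each update, and VoyaAnimMovement loops the VoyaMovement animation.
; Tick accumulates delta time into VoyaTime and writes it to the "Time" scalar of the MPC_VoyaTime parameter collection for materials to read.
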(event `self.ReceiveTick`
  (params (DeltaSeconds :type "Float (single-precision)"))
  ;[1 1 1] Activates time
  (bind _output_get (set `self.VoyaTime` (+ DeltaSeconds (`self.VoyaTime`))))
  (`KismetMaterialLibrary.SetScalarParameterValue` "/Game/VFX/VFX_Toolkit_V1/Materials/MPCollection/MPC_VoyaTime.MPC_VoyaTime" "Time" _output_get))

(event `/Game/VFX/VFX_Toolkit_V1/Blueprints/BP_SpawnSwirlyBeam.ReceiveBeginPlay`
  (`|ExecutionSequence`
    (:`then_0`
      (bind (_direction _arm1 _arm2) (`Timeline|Faketicker`)
        (:`Update`
          (`|ExecutionSequence`
            (:`then_0`
              (`SceneComponent.K2_AddLocalRotation` (`self.FairyArmMain`) (`KismetMathLibrary.MakeRotator` 0.0 0.0 _arm1) false false))
            (:`then_1`
              (`SceneComponent.K2_AddLocalRotation` (`self.FairyArm`) (`KismetMathLibrary.MakeRotator` 0.0 0.0 _arm2) false false))))))
    (:`then_1`
      (`SkeletalMeshComponent.PlayAnimation` (`self.VoyaAnimMovement`) "/Game/VFX/VFX_Toolkit_V1/SkeletalMeshes/AnimSeq/VoyaMovement.VoyaMovement" true))))

(fn `UserConstructionScript`)