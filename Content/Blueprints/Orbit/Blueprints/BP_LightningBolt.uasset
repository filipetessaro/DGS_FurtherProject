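; Procedural lightning bolt actor that strikes when BP_Orbit fires its lightning event, taking its origin, color, brightness and flicker settings from that actor.
; A fast looping timer line-traces downward in randomly jagged steps shaped by MPC_Lightning, adding spline mesh segments until a hit.
; A second timer flickers the bolt's visibility and the stratus cloud backlighting in sync, then destroys the actor after the maximum flicker count.
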(event `self.ReceiveBeginPlay`
  ;[1 1 1] Creation
  (for _index (range (+ (- (`SplineComponent.GetNumberOfSplinePoints` (`self.Spline`)) 2) 1))
    (set `self.PointCount` _index)
    ;[1 1 1] Tie Functionality to Orbit Controls
    (add `self.FireLightning` (delegate `Fire`))
    (bind _outactors (`GameplayStatics.GetAllActorsOfClass` "/Game/Blueprints/Orbit/Blueprints/BP_Orbit.BP_Orbit_C"))
    (set `self.BP_Orbit` (`|GetArrayItem` _outactors))))

(event `Fire`
  (bind _timer (`self.Timer`))
  ;[1 1 1] Controls
  (bind _returnvalue (`KismetSystemLibrary.K2_SetTimerDelegate` (delegate `LightningEvent`) 0.008 true))
  (set `self.Timer` _returnvalue)
  (if (`KismetSystemLibrary.K2_IsTimerPausedHandle` _timer)
    (`KismetSystemLibrary.K2_UnPauseTimerHandle` _timer)))

(event `LightningEvent`
  (bind _pointcount (`self.PointCount`))
  (bind (_location _tangent) (`SplineComponent.GetLocationAndTangentAtSplinePoint` (`self.Spline`) (+ _pointcount 1) "Local"))
  (bind (_location_2 _tangent_2) (`SplineComponent.GetLocationAndTangentAtSplinePoint` (`self.Spline`) (+ (- _pointcount 2) 1) "Local"))
  ;[1 1 1] Fire
  (if (`self.Loop`)
    (`|ExecutionSequence`
      (:`then_0`
        ;[1 1 1] Trace
        (`/Engine/EditorBlueprintResources/StandardMacros.DoOnce` false
          (:`Completed`
            (bind _output_get (set `self.Trace Start` (`/Game/Blueprints/Orbit/Blueprints/BP_Orbit.StrikeLocation` (`self.BP_Orbit`)))))))
      (:`then_1`
        _))
    (bind (_outhit _returnvalue) (`KismetSystemLibrary.LineTraceSingle` :`Start` _output_get :`End` (`self.LightningShape` (`self.Trace Start`)) :`TraceChannel` "TraceTypeQuery1" :`DrawTime` 1.0))
    ;[1 1 1] Hit causes reset
    (if _returnvalue
      (set `self.Loop` false)
      (`KismetSystemLibrary.PrintString` "Hit")
      (else
        (bind (_bblockinghit _binitialoverlap _time _distance _location_3 _impactpoint _normal _impactnormal _physmat _hitactor _hitcomponent _hitbonename _hititem _faceindex _tracestart _traceend) (`GameplayStatics.BreakHitResult` _outhit))
        ;[1 1 1] Build Spline
        (`SplineComponent.AddSplinePointAtIndex` (`self.Spline`) _traceend (`self.PointCount`) "Local" true)
        (set `self.Trace Start` _traceend)
        (bind _returnvalue_2 (`AddComponent|NODE_AddSplineMeshComponent-0` :`bManualAttachment` true))
        (bind _output_get_2 (set `self.SplineMesh` _returnvalue_2))
        (bind _returnvalue_3 (`PrimitiveComponent.CreateDynamicMaterialInstance` _output_get_2 0 (`PrimitiveComponent.GetMaterial` _output_get_2 0)))
        (`MaterialInstanceDynamic.SetVectorParameterValue` _returnvalue_3 "LightningColor" (`/Game/Blueprints/Orbit/Blueprints/BP_Orbit.Lightning Color` (`self.BP_Orbit`)))
        (`MaterialInstanceDynamic.SetScalarParameterValue` _returnvalue_3 "LightningIntensity" (`/Game/Blueprints/Orbit/Blueprints/BP_Orbit.Lightning Brightness` (`self.BP_Orbit`)))
        (set `self.MaximumFlickers` (`/Game/Blueprints/Orbit/Blueprints/BP_Orbit.Lightning Max Flickers` (`self.BP_Orbit`)))
        (`LightComponent.SetLightColor` (`self.StrikeFlash`) (`/Game/Blueprints/Orbit/Blueprints/BP_Orbit.Lightning Color` (`self.BP_Orbit`)) true)
        (`SceneComponent.K2_AttachToComponent` _output_get_2 (`self.DefaultSceneRoot`) "None" "KeepRelative" "KeepRelative" "KeepRelative" true)
        (`SplineMeshComponent.SetStartAndEnd` (`self.SplineMesh`) _location_2 _tangent_2 _location _tangent true)
        (`/Engine/EditorBlueprintResources/StandardMacros.DoOnce` false
          (:`Completed`
            (`KismetSystemLibrary.K2_SetTimerDelegate` (delegate `CustomEvent_0`) (`/Game/Blueprints/Orbit/Blueprints/BP_Orbit.Lightning Flicker Rate` (`self.BP_Orbit`)) true)))))))

(event `CustomEvent_0`
  (bind _bp_orbit (`self.BP_Orbit`))
  (bind _bp_orbit_2 (`self.BP_Orbit`))
  ;[1 1 1] Build Spline
  (`/Engine/EditorBlueprintResources/StandardMacros.FlipFlop`
    (:`A`
      (`SceneComponent.SetVisibility` (`self.DefaultSceneRoot`) false true)
      (set `/Game/Blueprints/Orbit/Blueprints/BP_Orbit.Lightning Intensity Exponent` 0.0 (`self.BP_Orbit`))
      (`MaterialInstanceDynamic.SetScalarParameterValue` (`/Game/Blueprints/Orbit/Blueprints/BP_Orbit.StratusMat` _bp_orbit) "Lightning Lighting Intensity" (* (`/Game/Blueprints/Orbit/Blueprints/BP_Orbit.Lightning Backlighting Intensity` _bp_orbit) (`/Game/Blueprints/Orbit/Blueprints/BP_Orbit.Lightning Intensity Exponent` _bp_orbit))))
    (:`B`
      (`SceneComponent.SetVisibility` (`self.DefaultSceneRoot`) true true)
      (set `/Game/Blueprints/Orbit/Blueprints/BP_Orbit.Lightning Intensity Exponent` 1.0 (`self.BP_Orbit`))
      (`MaterialInstanceDynamic.SetScalarParameterValue` (`/Game/Blueprints/Orbit/Blueprints/BP_Orbit.StratusMat` _bp_orbit_2) "Lightning Lighting Intensity" (* (`/Game/Blueprints/Orbit/Blueprints/BP_Orbit.Lightning Backlighting Intensity` _bp_orbit_2) (`/Game/Blueprints/Orbit/Blueprints/BP_Orbit.Lightning Intensity Exponent` _bp_orbit_2)))))
  (bind _output_get (set `self.FlickerCount` (+ (`self.FlickerCount`) 1)))
  (if (>= _output_get (`self.MaximumFlickers`))
    (`MaterialInstanceDynamic.SetScalarParameterValue` (`/Game/Blueprints/Orbit/Blueprints/BP_Orbit.StratusMat` (`self.BP_Orbit`)) "Lightning Lighting Intensity" 0.0)
    (`KismetSystemLibrary.Delay` 1.0)
    (`self.K2_DestroyActor`)))

(fn `LightningShape`
  (params (`Location In` :type "Vector Structure"))
  (returns (`Location Out` :type "Vector Structure"))
  (bind _returnvalue (`KismetMaterialLibrary.GetScalarParameterValue` "/Game/Blueprints/Orbit/Materials/ParameterCollections/MPC_Lightning.MPC_Lightning" "LightningBreakLengths"))
  (set `self.Bolt Trace Distance` _returnvalue)
  (bind _returnvalue_2 (`KismetMaterialLibrary.GetScalarParameterValue` "/Game/Blueprints/Orbit/Materials/ParameterCollections/MPC_Lightning.MPC_Lightning" "LightningArc"))
  (set `self.Bolt Arc Exponent` _returnvalue_2)
  (if (`KismetMathLibrary.InRange_FloatFloat` (`KismetMathLibrary.RandomFloatInRange` 0.0 1.0) 0.0 0.5)
    (set `self.Pos/Neg` 1.0)
    (else
      (set `self.Pos/Neg` -1.0)))
  (return (`KismetMathLibrary.MakeVector` (+ (.x `Location In`) (* (`self.Bolt Arc Exponent`) (`self.Pos/Neg`))) (+ (.y `Location In`) (* (`self.Bolt Arc Exponent`) (`self.Pos/Neg`))) (- (.z `Location In`) (`self.Bolt Trace Distance`)))))

(fn `UserConstructionScript`
  (for _index (range (+ (- (`SplineComponent.GetNumberOfSplinePoints` (`self.Spline`)) 2) 1))
    (bind _output_get (set `self.PointCount` _index))
    (bind _returnvalue (`AddComponent|NODE_AddSplineMeshComponent-1` :`bManualAttachment` true))
    (`SceneComponent.K2_AttachToComponent` _returnvalue (`self.DefaultSceneRoot`) "None" "KeepRelative" "KeepRelative" "KeepRelative" true)
    (bind (_location _tangent) (`SplineComponent.GetLocationAndTangentAtSplinePoint` (`self.Spline`) _output_get "Local"))
    (bind (_location_2 _tangent_2) (`SplineComponent.GetLocationAndTangentAtSplinePoint` (`self.Spline`) (+ _output_get 1) "Local"))
    (`SplineMeshComponent.SetStartAndEnd` _returnvalue _location _tangent _location_2 _tangent_2 true)))