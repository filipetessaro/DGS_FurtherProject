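; Component for a BP_BaseCharacter owner that manages health and stamina regeneration, damage and death.
; Looping timers started by the owner add clamped amounts to SActorData; a timed stop is intended for temporary regen, but stamina's delay is zero.
; OnDamage adds its signed amount to health, then DeathCheck clears both regen timers on every hit.
; At zero health it halts movement, disables input and shows the GameInstance death screen after a delay.
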(event `self.ReceiveBeginPlay`
  (bind _asbp_base_character (cast `/Game/Blueprints/BP_BaseCharacter` (`self.GetOwner`)))
  (set `self.OwnerBaseCharacter` _asbp_base_character))

(event `InterruptHealthRegen`
  ;[0 1 0] Start Health Regen Tick
  (`self.StopHealthRegen`))

(event `StartHealthRegen`
  (params (`TemporaryRegen?` :type Boolean :default false) (TimeToLast :type "Float (double-precision)" :default 5.0))
  ;[0 1 0] Start Health Regen Tick
  (`self.OnHealthRegenStarted`) ; this can be used by the owner to add additional behaviors
  (set `self.TemporaryTimeHealthRegen` TimeToLast)
  (set `self.TemporaryHealthRegen?` `TemporaryRegen?`)
  (`KismetSystemLibrary.K2_ClearAndInvalidateTimerHandle` (`self.HealthRegenHandle`))
  (if (`self.TemporaryHealthRegen?`)
    (`KismetSystemLibrary.K2_SetTimerDelegate` (delegate `InterruptHealthRegen`) (`self.TemporaryTimeHealthRegen`)))
  (bind _returnvalue (`KismetSystemLibrary.K2_SetTimer` null "HealthRegen" (`.HealthRegenRate_11_BDBE9DA04253252B534AE089BFC70657` (break `/Game/Blueprints/Datas/S_ActorData` (`self.S_ActorData`))) true))
  (set `self.HealthRegenHandle` _returnvalue))

(event `StopHealthRegen`
  (bind _healthregenhandle (`self.HealthRegenHandle`))
  ;[0 1 0] Stop Health Regen tick
  (`self.OnHealthRegenStoped`) ; this can be used by the owner to add additional behaviors
  (`KismetSystemLibrary.K2_PauseTimerHandle` _healthregenhandle)
  (`KismetSystemLibrary.K2_ClearAndInvalidateTimerHandle` _healthregenhandle))

(event `InterruptStaminaRegen`
  ;[1 1 0] Start stamina Regen
  (`self.StopStaminaRegen`))

(event `StartStaminaRegen`
  (params (`TemporaryRegen?` :type Boolean) (TimeToLast :type "Float (double-precision)" :default 5.0))
  ;[1 1 0] Start stamina Regen
  (`self.OnStaminaRegenStarted`)
  (set `self.TemporaryStaminaRegen?` `TemporaryRegen?`)
  (set `self.TemporaryTimeStaminaRegen` TimeToLast)
  (`KismetSystemLibrary.K2_ClearAndInvalidateTimerHandle` (`self.StaminaRegenHandle`))
  (if (`self.TemporaryStaminaRegen?`)
    (`KismetSystemLibrary.K2_SetTimerDelegate` (delegate `InterruptStaminaRegen`)))
  (bind _returnvalue (`KismetSystemLibrary.K2_SetTimer` null "StaminaRegen" (`.StaminaRegenRate_12_0530AD574B2286417ADB43BE1A87DCEC` (break `/Game/Blueprints/Datas/S_ActorData` (`self.S_ActorData`))) true))
  (set `self.StaminaRegenHandle` _returnvalue))

(event `StopStaminaRegen`
  (bind _staminaregenhandle (`self.StaminaRegenHandle`))
  ;[1 1 0] Stop stamina Regen
  (`self.OnStaminaRegenStoped`)
  (`KismetSystemLibrary.K2_PauseTimerHandle` _staminaregenhandle)
  (`KismetSystemLibrary.K2_ClearAndInvalidateTimerHandle` _staminaregenhandle))

(fn `DeathCheck`
  (locals (TimerHandleDeath :type "TimerHandle Structure"))
  (bind _s_actordata (`self.S_ActorData`))
  (bind _ownerbasecharacter (`self.OwnerBaseCharacter`))
  (`KismetSystemLibrary.K2_ClearAndInvalidateTimerHandle` (`self.HealthRegenHandle`))
  (`KismetSystemLibrary.K2_ClearAndInvalidateTimerHandle` (`self.StaminaRegenHandle`))
  (`KismetSystemLibrary.K2_ClearAndInvalidateTimerHandle` (`local.TimerHandleDeath`))
  (if (<= (`.ActualHealth_6_6CD5CF1B43B8F038E7AC4F9CFB9F9BEB` (break `/Game/Blueprints/Datas/S_ActorData` _s_actordata)) 0.0)
    (setmembers `/Game/Blueprints/Datas/S_ActorData` :`StructRef` _s_actordata :`IsDead?` true)
    (`MovementComponent.StopMovementImmediately` (`Character.CharacterMovement` _ownerbasecharacter))
    (`Actor.DisableInput` _ownerbasecharacter (`GameplayStatics.GetPlayerController` 0))
    (bind _returnvalue (`KismetSystemLibrary.K2_SetTimer` null "DeathEventScreen" 2.5))
    (set `local.TimerHandleDeath` _returnvalue)
    (return)))

(fn `DeathEventScreen`
  (bind _asf_game_instance (cast `/Game/Blueprints/Core/F_GameInstance` (`GameplayStatics.GetGameInstance`)))
  (`/Game/Blueprints/Core/F_GameInstance.AddDeathScreen` _asf_game_instance)
  (return))

(fn `HealthRegen`
  (bind _s_actordata (`self.S_ActorData`))
  (bind (_maxhealth _actualhealth _maxstamina _actualstamina _healthregenrate _staminaregenrate _healthregenamount) (break `/Game/Blueprints/Datas/S_ActorData` _s_actordata))
  (setmembers `/Game/Blueprints/Datas/S_ActorData` :`StructRef` _s_actordata :`ActualHealth` (`KismetMathLibrary.FClamp` (+ _actualhealth _healthregenamount) 0.0 _maxhealth))
  (return))

(fn `OnDamage`
  (params (AmountToDamage :type "Float (double-precision)"))
  (bind _s_actordata (`self.S_ActorData`))
  (bind (_maxhealth _actualhealth) (break `/Game/Blueprints/Datas/S_ActorData` _s_actordata))
  (setmembers `/Game/Blueprints/Datas/S_ActorData` :`StructRef` _s_actordata :`ActualHealth` (`KismetMathLibrary.FClamp` (+ _actualhealth AmountToDamage) 0.0 _maxhealth))
  (`self.DeathCheck`)
  (`self.OnDamagePlayer`)
  (return))

(fn `RestoreHealth`
  (params (AmountToRestore :type "Float (double-precision)"))
  (bind _s_actordata (`self.S_ActorData`))
  (bind (_maxhealth _actualhealth) (break `/Game/Blueprints/Datas/S_ActorData` _s_actordata))
  (setmembers `/Game/Blueprints/Datas/S_ActorData` :`StructRef` _s_actordata :`ActualHealth` (`KismetMathLibrary.FClamp` (+ _actualhealth AmountToRestore) 0.0 _maxhealth))
  (return))

(fn `RestoreStamina`
  (params (AmountToRestore :type "Float (double-precision)"))
  (bind _s_actordata (`self.S_ActorData`))
  (bind (_maxhealth _actualhealth _maxstamina _actualstamina) (break `/Game/Blueprints/Datas/S_ActorData` _s_actordata))
  (setmembers `/Game/Blueprints/Datas/S_ActorData` :`StructRef` _s_actordata :`ActualStamina` (`KismetMathLibrary.FClamp` (+ _actualstamina AmountToRestore) 0.0 _maxstamina))
  (return))

(fn `StaminaRegen`
  (bind _s_actordata (`self.S_ActorData`))
  (bind (_maxhealth _actualhealth _maxstamina _actualstamina _healthregenrate _staminaregenrate _healthregenamount _staminaregenamount) (break `/Game/Blueprints/Datas/S_ActorData` _s_actordata))
  (setmembers `/Game/Blueprints/Datas/S_ActorData` :`StructRef` _s_actordata :`ActualStamina` (`KismetMathLibrary.FClamp` (+ _actualstamina _staminaregenamount) 0.0 _maxstamina))
  (return))