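; Base door that swings its mesh on yaw, opened and closed by BP_BaseCharacter interaction or automatically by proximity.
; The collision box binds the character's OnInteract, gates it with CanInteract, and toggles a "Press E" widget.
; With ShouldAutoClose, overlap begin and end retarget an interpolated rotation.
; Interaction steps yaw by DoorSpeed until near the open or closed angle, both modes using start/stop custom ticks.
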(event `SetMessageVisible`
  (`SceneComponent.SetVisibility` (`self.Widget`) true false))

(event `self.ReceiveBeginPlay`
  (bind _asw_item_message (cast `/Game/Blueprints/Inventory/W_ItemMessage` (`WidgetComponent.GetUserWidgetObject` (`self.Widget`))))
  (set `/Game/Blueprints/Inventory/W_ItemMessage.TextToShow` "Press \"E\" To Open / Close" _asw_item_message))

(event `SetMessageInvisible`
  (`SceneComponent.SetVisibility` (`self.Widget`) false false))

(event `self.Box collison.OnComponentBeginOverlap`
  (params (OverlappedComponent :type "PrimitiveComponent Object Reference") (OtherActor :type "Actor Object Reference") (OtherComp :type "PrimitiveComponent Object Reference") (OtherBodyIndex :type Integer) (bFromSweep :type Boolean) (SweepResult :type "HitResult Structure (by ref)"))
  (bind _asbp_base_character (cast `/Game/Blueprints/BP_BaseCharacter` OtherActor))
  (bind _output_get (set `self.BaseCharRef` _asbp_base_character))
  (add `/Game/Blueprints/BP_BaseCharacter.OnInteract` _output_get (delegate `OnInteract_Event_0`))
  (set `self.CanInteract?` true)
  (if (`Pawn.IsLocallyControlled` (`self.BaseCharRef`))
    (`self.SetMessageVisible`))
  (if (`self.ShouldAutoClose?`)
    (`self.StartOpenningDoor(Auto)`)))

(event `self.Box collison.OnComponentEndOverlap`
  (params (OverlappedComponent :type "PrimitiveComponent Object Reference") (OtherActor :type "Actor Object Reference") (OtherComp :type "PrimitiveComponent Object Reference") (OtherBodyIndex :type Integer))
  (cast `/Game/Blueprints/BP_BaseCharacter` OtherActor)
  (`self.SetMessageInvisible`)
  (set `self.CanInteract?` false)
  (if (`self.ShouldAutoClose?`)
    (`self.StartClosingDoor(Auto)`)))

(event `OnInteract_Event_0`
  (if (`self.CanInteract?`)
    (`self.StartMovingDoor(NonAuto)`)))

(event `StartOpenningDoor(Auto)`
  (bind _doormesh (`self.DoorMesh`))
  (bind (_relativerotation_roll _relativerotation_pitch _relativerotation_yaw) (`KismetMathLibrary.BreakRotator` (`SceneComponent.RelativeRotation` _doormesh)))
  ;[1 1 1] Actual auto system
  (set `self.OpeningTarget` (`self.AngleToOpen`))
  (`/Game/Blueprints/BML_GeneralMacros.ML_CustomTick` 0.0 :!label _label
    (:`then`
      (`SceneComponent.K2_SetRelativeRotation` _doormesh (`KismetMathLibrary.MakeRotator` _relativerotation_roll _relativerotation_pitch (`KismetMathLibrary.FInterpTo` _relativerotation_yaw (`self.OpeningTarget`) (`GameplayStatics.GetWorldDeltaSeconds`) 1.0)) false false)
      (if (`KismetMathLibrary.NearlyEqual_FloatFloat` _relativerotation_yaw (`self.OpeningTarget`) 0.1)
        (`self.CustomTickStop`)))))

(event `CustomTickStop`
  ;[1 1 1] Actual auto system
  (goto _label :!via `Stop`))

(event `StartClosingDoor(Auto)`
  ;[1 1 1] Actual auto system
  (set `self.OpeningTarget` (`self.AngleToClose`))
  (`self.CustomTickStop`)
  (goto _label))

(event `StartMovingDoor(NonAuto)`
  (bind _doormesh (`self.DoorMesh`))
  (bind _doorspeed (`self.DoorSpeed`))
  (bind (_relativerotation_roll _relativerotation_pitch _relativerotation_yaw) (`KismetMathLibrary.BreakRotator` (`SceneComponent.RelativeRotation` _doormesh)))
  ;[1 1 1] Alternative setup, that can be used
  ; needs to be linked to interact system
  ; to have a better behavior and more intuitive for the player
  (set `self.ReallyFinished` false)
  (if (`self.DoorIsOpen`)
    (set `self.ValueToAdd` (* _doorspeed -1.0))
    (set `self.IsOpenning?` false)
    (else
      (set `self.ValueToAdd` _doorspeed)
      (set `self.IsOpenning?` true)))
  (`/Game/Blueprints/BML_GeneralMacros.ML_CustomTick` 0.0 :!label _label_2
    (:`then`
      (set `self.OpeningTarget` (+ _relativerotation_yaw (`self.ValueToAdd`)))
      (`SceneComponent.K2_SetRelativeRotation` _doormesh (`KismetMathLibrary.MakeRotator` _relativerotation_roll _relativerotation_pitch (`KismetMathLibrary.FInterpTo` _relativerotation_yaw (`self.OpeningTarget`) (`GameplayStatics.GetWorldDeltaSeconds`) 120.0)) false false)
      (if (`self.IsOpenning?`)
        (set `self.WhatToCheck` (`self.AngleToOpen`))
        (else
          (set `self.WhatToCheck` (`self.AngleToClose`))))
      (if (`KismetMathLibrary.NearlyEqual_FloatFloat` _relativerotation_yaw (`self.WhatToCheck`) 5.0)
        (set `self.ReallyFinished` true)
        (`self.TickStop(NonAuto)`)))
    (:`Stopped`
      (if (`self.ReallyFinished`)
        (if (`self.IsOpenning?`)
          (set `self.DoorIsOpen` true)
          (else
            (set `self.DoorIsOpen` false)))))))

(event `TickStop(NonAuto)`
  ;[1 1 1] Alternative setup, that can be used
  ; needs to be linked to interact system
  ; to have a better behavior and more intuitive for the player
  (goto _label_2 :!via `Stop`))

(fn `UserConstructionScript`)