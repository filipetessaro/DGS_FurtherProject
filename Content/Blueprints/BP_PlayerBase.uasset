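; Base player character handling movement, first/third-person camera toggle, zoom and merchant trading.
; BeginPlay starts health and stamina regen on authority, adds itself to the scene capture and sets game-only input.
; Inventory, merchant and inspection flags gate movement, look and zoom, with zoom also driving the book-reading widget.
; Buying checks money and encumbrance, selling pays half price, and NumPad 2 launches the character upward.
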(event `self.ReceiveBeginPlay`
  (bind _returnvalue (`GameplayStatics.GetPlayerController` 0))
  (bind _healthstaminacomponent (`self.HealthStaminaComponent`))
  ;[1 1 1] Begin play to initiate Regen functions and add HUD
  (`parent.ReceiveBeginPlay`)
  (`/Engine/EditorBlueprintResources/ActorMacros.Switch Has Authority`
    (:`Authority`
      (`/Game/Blueprints/BPC_RegenComponent.StartHealthRegen` _healthstaminacomponent false 5.0)
      (`/Game/Blueprints/BPC_RegenComponent.StartStaminaRegen` _healthstaminacomponent false 5.0))
    (:`Remote`
      _))
  (`KismetArrayLibrary.Array_Add` (`SceneCaptureComponent.ShowOnlyActors` (`self.SceneCaptureComponent2D`)) self)
  (`KismetSystemLibrary.Delay` 0.2)
  (set `PlayerController.bShowMouseCursor` false _returnvalue)
  (`WidgetBlueprintLibrary.SetInputMode_GameOnly` _returnvalue))

(event `InputAxis|MoveForward`
  (params (AxisValue :type "Float (single-precision)"))
  ;[1 1 1] Player movement
  (if (not (or (`self.InventoryOpened?`) (`self.MerchantOpened?`)))
    (`self.AddMovementInput` (`KismetMathLibrary.GetForwardVector` (`KismetMathLibrary.MakeRotator` 0.0 0.0 (.yaw (`self.GetControlRotation`)))) AxisValue)))

(event `InputAction|ToggleCamera`
  (params (Key :type "Key Structure"))
  (bind _camera (`self.Camera`))
  ;[1 1 1] Camera toggle
  (:`Pressed`
    (if (`self.IsThirdPerson?`)
      (set `self.IsThirdPerson?` false)
      (`SceneComponent.K2_AttachToComponent` _camera (`self.FirstPersonArm`) "None" "SnapToTarget" "SnapToTarget" "KeepRelative" true)
      (set `self.bUseControllerRotationYaw` true)
      (else
        (set `self.IsThirdPerson?` true)
        (`SceneComponent.K2_AttachToComponent` _camera (`self.ThirdPersonArm`) "None" "SnapToTarget" "SnapToTarget" "KeepRelative" true)
        (set `self.bUseControllerRotationYaw` false)))))

(event `InputAxis|MoveRight`
  (params (AxisValue :type "Float (single-precision)"))
  ;[1 1 1] Player movement
  (if (not (or (`self.InventoryOpened?`) (`self.MerchantOpened?`)))
    (`self.AddMovementInput` (`KismetMathLibrary.GetRightVector` (`KismetMathLibrary.MakeRotator` 0.0 0.0 (.yaw (`self.GetControlRotation`)))) AxisValue)))

(event `InputAxis|Turn`
  (params (AxisValue :type "Float (single-precision)"))
  ;[1 1 1] Player movement
  (bind _output_get (set `self.LeftRightScale` AxisValue))
  (if (not (`self.Inspecting/ReadingItem?`))
    (`self.AddControllerYawInput` _output_get)))

(event `InputAxis|LookUp`
  (params (AxisValue :type "Float (single-precision)"))
  ;[1 1 1] Player movement
  (bind _output_get (set `self.UpDownScale` AxisValue))
  (if (not (`self.Inspecting/ReadingItem?`))
    (`self.AddControllerPitchInput` _output_get)))

(event `InputAction|ZoomIn`
  (params (Key :type "Key Structure"))
  (bind _thirdpersonarm (`self.ThirdPersonArm`))
  (bind _w_bookreadwidget (`/Game/Blueprints/Core/F_GameInstance.W_BookReadWidget` (`self.GameInstanceRef`)))
  ;[1 1 1] TP Zoom / Book zoom
  (:`Pressed`
    (if (`self.IsThirdPerson?`)
      (if (not (`self.MerchantOpened?`))
        (set `self.Zoom` (`KismetMathLibrary.FClamp` (- (`self.Zoom`) 10.0) 120.0 300.0))
        (if (`self.InventoryOpened?`)
          (`/Engine/EditorBlueprintResources/StandardMacros.IsValid` _w_bookreadwidget :!label _label
            (:`Is Valid`
              (`/Game/Blueprints/Inventory/W_BookReadInspectView.ZoomIn/Out` _w_bookreadwidget (`self.Zoom`))))
          (else
            (set `SpringArmComponent.TargetArmLength` (`KismetMathLibrary.FClamp` (- (`SpringArmComponent.TargetArmLength` _thirdpersonarm) 10.0) 50.0 600.0) _thirdpersonarm)))))))

(event `InputAction|Jump`
  (params (Key :type "Key Structure"))
  ;[1 1 1] Player movement
  (:`Pressed`
    (`self.Jump`)))

(event `InputAction|ZoomOut`
  (params (Key :type "Key Structure"))
  (bind _thirdpersonarm (`self.ThirdPersonArm`))
  ;[1 1 1] TP Zoom / Book zoom
  (:`Pressed`
    (if (`self.IsThirdPerson?`)
      (if (not (`self.MerchantOpened?`))
        ;;[1 1 1] for the read book
        (set `self.Zoom` (`KismetMathLibrary.FClamp` (+ (`self.Zoom`) 10.0) 120.0 300.0))
        (if (`self.InventoryOpened?`)
          (goto _label)
          (else
            (set `SpringArmComponent.TargetArmLength` (`KismetMathLibrary.FClamp` (+ (`SpringArmComponent.TargetArmLength` _thirdpersonarm) 10.0) 50.0 600.0) _thirdpersonarm)))))))

(event `Key|NumPadTwo`
  (params (Key :type "Key Structure"))
  (:`Pressed`
    (`self.LaunchCharacter` (0.0 0.0 2000.0) false true)))

(fn `PlayerBuyItem`
  (params (Item :type "/Game/Blueprints/items/S_ItemData Structure"))
  (bind (_itemname _itemdescription _icon _questitem_ _itemtype _isstackable_ _weight _pricevalue) (break `/Game/Blueprints/items/S_ItemData` Item))
  (bind _s_characterdata (`self.S_CharacterData`))
  (bind (_charname _charicon _encumbance _totalweight _level _experience _money) (break `/Game/Blueprints/Datas/S_CharacterData` _s_characterdata))
  (if (>= _money _pricevalue)
    (if (>= _totalweight _encumbance)
      (`KismetSystemLibrary.PrintString` "YOU ARE TOO HEAVY")
      (else
        (setmembers `/Game/Blueprints/Datas/S_CharacterData` :`StructRef` _s_characterdata :`Money` (`KismetMathLibrary.FClamp` (- _money _pricevalue) 0.0 1000000000.0))
        (`self.AddSpecificItemToInventory` Item)
        (`self.ExternalUpdateInventory/Merchant`)))
    (else
      (`KismetSystemLibrary.PrintString` "YOU DON´T HAVE ENOUGHT MONEY")))
  (return))

(fn `PlayerSellItem`
  (params (Item :type "Array of /Game/Blueprints/items/S_ItemData Structure") (Index :type Integer) (ItemWeight :type "Float (double-precision)") (PriceValue :type "Float (double-precision)"))
  (bind _s_characterdata (`self.S_CharacterData`))
  (setmembers `/Game/Blueprints/Datas/S_CharacterData` :`StructRef` _s_characterdata :`Money` (+ (`.Money_22_20A961FB4A1B2AF9B1C6E28385C73C60` (break `/Game/Blueprints/Datas/S_CharacterData` _s_characterdata)) (/ PriceValue 2.0)))
  (`self.RemoveItemFromInventory` Item Index ItemWeight)
  (`self.ExternalUpdateInventory/Merchant`)
  (return))

(fn `UserConstructionScript`)